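; BP_Poignee_Grab is a grab handle that gives visual feedback when overlapped or selected.
; The construction script applies a configurable mesh, and BeginPlay creates a dynamic instance of the handle material.
; The Changer_Etat event takes overlap and selection states and updates the material only when either changes.
; Overlap drives the highlight intensity parameter, while selection switches the base color.
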(event `self.ReceiveBeginPlay`
  (bind _returnvalue (`PrimitiveComponent.CreateDynamicMaterialInstance` (`self.Mesh_poignee`) 0 "/Game/Briques_projets/Grab/MA_Poignee.MA_Poignee" "None"))
  (set `self.Matiere_poignee` _returnvalue))

(event `Changer_Etat`
  (params (overlap :type Boolean) (Selection :type Boolean))
  (bind _matiere_poignee (`self.Matiere_poignee`))
  (bind _matiere_poignee_2 (`self.Matiere_poignee`))
  (`|ExecutionSequence`
    (:`then_0`
      (if (not (== overlap (`self.Est_overlap`)))
        (bind _output_get (set `self.Est_overlap` overlap))
        (if _output_get
          (`MaterialInstanceDynamic.SetScalarParameterValue` _matiere_poignee_2 "Intensite_selection" 3.0)
          (else
            (`MaterialInstanceDynamic.SetScalarParameterValue` _matiere_poignee_2 "Intensite_selection" 0.0)))))
    (:`then_1`
      (if (not (== Selection (`self.Est_Selectionne`)))
        (bind _output_get_2 (set `self.Est_Selectionne` Selection))
        (if _output_get_2
          (`MaterialInstanceDynamic.SetVectorParameterValue` _matiere_poignee "Couleur_base" (`KismetMathLibrary.MakeColor` 0.05 0.13))
          (else
            (`MaterialInstanceDynamic.SetVectorParameterValue` _matiere_poignee "Couleur_base" (`KismetMathLibrary.MakeColor` 0.41 0.48 0.75))))))))

(fn `UserConstructionScript`
  (`StaticMeshComponent.SetStaticMesh` (`self.Mesh_poignee`) (`self.Maillage_poignee`)))