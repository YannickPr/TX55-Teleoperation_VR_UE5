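; VR grab handle actor that moves a target object, itself by default, with the component grabbing it.
; UseHandle stores the start and relative transforms and swaps the sphere's material for grab state.
; While grabbed in VR, Tick offers the position to a BPi_Grab receiver, applying the composed transform if unhandled.
; Without a headset, Tick sends the sphere's position for debugging; ResetHandled restores the pre-grab transform.
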(event `Initialisation`
  (params (`Object to move` :type "Actor Object Reference") (CAO :type "StaticMesh Object Reference") (Transform :type "Transform Structure") (`Send info to` :type "Actor Object Reference"))
  (bind _sphere (`self.Sphere`))
  (`|ExecutionSequence`
    (:`then_0`
      (`/Engine/EditorBlueprintResources/StandardMacros.IsValid` `Object to move`
        (:`Is Valid`
          (set `self.Object To Move` `Object to move`))
        (:`Is Not Valid`
          (set `self.Object To Move` self))))
    (:`then_1`
      (`/Engine/EditorBlueprintResources/StandardMacros.IsValid` CAO
        (:`Is Valid`
          (`StaticMeshComponent.SetStaticMesh` (`self.Sphere`) CAO))))
    (:`then_2`
      (`SceneComponent.K2_SetRelativeTransform` _sphere Transform false false)
      (`PrimitiveComponent.SetMaterial` _sphere 0 (`self.Material base`)))
    (:`then_3`
      (set `self.Send info to` `Send info to`))))

(event `self.ReceiveBeginPlay`
  (if (`HeadMountedDisplayFunctionLibrary.IsHeadMountedDisplayEnabled`)
    _))

(event `self.ReceiveTick`
  (params (DeltaSeconds :type "Float (single-precision)"))
  (bind _send_info_to (`self.Send info to`))
  (if (`HeadMountedDisplayFunctionLibrary.IsHeadMountedDisplayEnabled`)
    (if (`self.Is grabbed`)
      (if (and (`KismetSystemLibrary.IsValid` _send_info_to) (`KismetSystemLibrary.DoesImplementInterface` _send_info_to "/Game/Briques_projets/Grab/Handle_v2/BPi_Grab.BPi_Grab_C"))
        (bind _controlled_by_target (message `/Game/Briques_projets/Grab/Handle_v2/BPi_Grab.Communicate_data_handle` (`self.Send info to`) (+ (`SceneComponent.K2_GetComponentLocation` (`self.Grabed By`)) (`self.Relative Position`)) (struct) self (`self.Object To Move`)))
        (if (not _controlled_by_target)
          (`self.K2_SetActorTransform` (`self.Object To Move`) (`KismetMathLibrary.ComposeTransforms` (`self.Relative transform`) (`SceneComponent.K2_GetComponentToWorld` (`self.Grabed By`))) false false :!label _label))
        (else
          (goto _label))))
    (else
      ;[1 1 1] for debug from pc
      (message `/Game/Briques_projets/Grab/Handle_v2/BPi_Grab.Communicate_data_handle` (`self.Send info to`) (`SceneComponent.K2_GetComponentLocation` (`self.Sphere`)) (struct) self (`self.Object To Move`)))))

(event `self.Reset_handled`
  (`self.K2_SetActorTransform` (`self.Object To Move`) (`self.Init grab`) false false)
  (`self.Use_handle` false))

(fn `Apply Transform`
  (params (`Grabbed by` :type "Transform Structure (by ref)") (`Initial relative transform` :type "Transform Structure (by ref)"))
  (returns (ReturnValue :type "Transform Structure"))
  (bind _rotation (.rotation `Initial relative transform`))
  (bind (_x _y _z) (`KismetMathLibrary.GetAxes` _rotation))
  (return (`KismetMathLibrary.MakeTransform` (+ (* (.x (.location `Initial relative transform`)) _x) (* (.y (.location `Initial relative transform`)) _y) (* (.z (.location `Initial relative transform`)) _z)) (`KismetMathLibrary.ComposeRotators` (.rotation `Grabbed by`) _rotation))))

(fn `Communicate_data_handle`
  (params (Position :type "Vector Structure") (Rotation :type "Rotator Structure") (`Ref handle` :type "/Game/Briques_projets/Grab/Handle_v2/BP_handle_v2 Object Reference") (`Object to move` :type "Actor Object Reference"))
  (returns (`Controlled by target` :type Boolean))
  (return false))

(fn `Get_handle_details`
  (returns (`Is grabbable` :type Boolean) (`Is Grabbed` :type Boolean))
  (return (`self.Is Grabbable`) (`self.Is grabbed`)))

(fn `Use_handle`
  (params (Grabbed :type Boolean) (`Is selected` :type Boolean) (`Grabed by` :type "StaticMeshComponent Object Reference"))
  (returns (`Object to move` :type "Actor Object Reference") (`Handle's target` :type "Actor Object Reference"))
  (bind _rootcomponent (`Actor.RootComponent` (`self.Object To Move`)))
  (bind _returnvalue (`SceneComponent.K2_GetComponentToWorld` _rootcomponent))
  (if Grabbed
    (set `self.Is grabbed` true)
    (`PrimitiveComponent.SetMaterial` (`self.Sphere`) 0 (`self.Material selected`))
    (set `self.Init grab` _returnvalue)
    (set `self.Grabed By` `Grabed by`)
    (set `self.Relative Position` (- (`SceneComponent.K2_GetComponentLocation` _rootcomponent) (`SceneComponent.K2_GetComponentLocation` `Grabed by`)))
    (set `self.Relative transform` (`KismetMathLibrary.ConvertTransformToRelative` (`SceneComponent.K2_GetComponentToWorld` `Grabed by`) _returnvalue))
    (else
      (set `self.Is grabbed` false)
      (if `Is selected`
        (`PrimitiveComponent.SetMaterial` (`self.Sphere`) 0 (`self.Material overlaped`))
        (else
          (`PrimitiveComponent.SetMaterial` (`self.Sphere`) 0 (`self.Material base`))))))
  (return (`self.Object To Move`) (`self.Send info to`)))

(fn `UserConstructionScript`
  (`self.Initialisation` (`self.Object To Move`) (`self.CAO`) (`self.Transform handle`) (`self.Send info to`)))