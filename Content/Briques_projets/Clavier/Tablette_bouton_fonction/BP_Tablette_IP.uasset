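; VR keypad tablet for editing the IP address stored in the Kinect server's parameters.
; Fingertip overlaps on digit, dot, delete, clear and OK keys go through a press-direction check, then reach GestionBouton via BPI_bouton to edit the length-capped string.
; Accepted or rejected presses drive controller haptics, sound, material swap and spline-defined key travel.
; OK sends the IP with the existing Kinect parameters to BPTablette, then destroys the keypad.
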(event `/Game/Briques_projets_rg2/Joueur/BPI_Interractions_VR.APressed`
  (params (`Handle used` :type "Actor Object Reference"))
  ;[1 1 1] pas de poignée actuellement
  (`self.Gestion bouton` "NewEnumerator1"))

(event `/Game/Briques_projets_rg2/Joueur/BPI_Interractions_VR.BPressed`
  (params (`Handle used` :type "Actor Object Reference"))
  ;[1 1 1] pas de poignée actuellement
  (`self.K2_DestroyActor`))

(event `self.ReceiveDestroyed`
  (`self.K2_DestroyActor` (`self.Handle`)))

(event `self.ReceiveBeginPlay`
  (bind (_parameters_kinect_lmin _parameters_kinect_lmax _parameters_kinect_hmin _parameters_kinect_hmax _parameters_kinect_dmin _parameters_kinect_dmax _parameters_kinect_nbvalmoy _parameters_kinect_simplification _parameters_kinect_ip) (break `/Game/Briques_projets_rg2/Kinect_webserver/STR_Param_kinect` (`/Game/Briques_projets_rg2/Kinect_webserver/BP_serveur_kinect.Parameters kinect` (`self.Serveur kinect`))))
  (`KismetSystemLibrary.Delay` 0.0) ; wait one frame
  (bind _output_get (set `self.IP writed` _parameters_kinect_ip))
  (`TextRenderComponent.K2_SetText` (`self.IP`) (`KismetTextLibrary.Conv_StringToText` _output_get)))

(event `self.Zone_overlap_supr.OnComponentBeginOverlap`
  (params (OverlappedComponent :type "PrimitiveComponent Object Reference") (OtherActor :type "Actor Object Reference") (OtherComp :type "PrimitiveComponent Object Reference") (OtherBodyIndex :type Integer) (bFromSweep :type Boolean) (SweepResult :type "HitResult Structure (by ref)"))
  (`self.Gerer_bouton` self "NewEnumerator2" "" OtherActor (`self.bouton supr`) (`self.Move supr`)))

(event `self.Zone_overlap_num 0.OnComponentBeginOverlap`
  (params (OverlappedComponent :type "PrimitiveComponent Object Reference") (OtherActor :type "Actor Object Reference") (OtherComp :type "PrimitiveComponent Object Reference") (OtherBodyIndex :type Integer) (bFromSweep :type Boolean) (SweepResult :type "HitResult Structure (by ref)"))
  ;[1 1 1] Num
  (`self.Gerer_bouton` self "NewEnumerator0" "0" OtherActor (`self.bouton num 0`) (`self.Move num 0`)))

(event `self.Zone_overlap_ok.OnComponentBeginOverlap`
  (params (OverlappedComponent :type "PrimitiveComponent Object Reference") (OtherActor :type "Actor Object Reference") (OtherComp :type "PrimitiveComponent Object Reference") (OtherBodyIndex :type Integer) (bFromSweep :type Boolean) (SweepResult :type "HitResult Structure (by ref)"))
  (`self.Gerer_bouton` self "NewEnumerator1" "" OtherActor (`self.bouton ok`) (`self.Move ok`)))

(event `self.Zone_overlap_num 1.OnComponentBeginOverlap`
  (params (OverlappedComponent :type "PrimitiveComponent Object Reference") (OtherActor :type "Actor Object Reference") (OtherComp :type "PrimitiveComponent Object Reference") (OtherBodyIndex :type Integer) (bFromSweep :type Boolean) (SweepResult :type "HitResult Structure (by ref)"))
  ;[1 1 1] Num
  (`self.Gerer_bouton` self "NewEnumerator0" "1" OtherActor (`self.bouton num 1`) (`self.Move num 1`)))

(event `self.Zone_overlap_supr2.OnComponentBeginOverlap`
  (params (OverlappedComponent :type "PrimitiveComponent Object Reference") (OtherActor :type "Actor Object Reference") (OtherComp :type "PrimitiveComponent Object Reference") (OtherBodyIndex :type Integer) (bFromSweep :type Boolean) (SweepResult :type "HitResult Structure (by ref)"))
  (`self.Gerer_bouton` self "NewEnumerator3" "" OtherActor (`self.bouton supr2`) (`self.Move supr2`)))

(event `self.Zone_overlap_num 2.OnComponentBeginOverlap`
  (params (OverlappedComponent :type "PrimitiveComponent Object Reference") (OtherActor :type "Actor Object Reference") (OtherComp :type "PrimitiveComponent Object Reference") (OtherBodyIndex :type Integer) (bFromSweep :type Boolean) (SweepResult :type "HitResult Structure (by ref)"))
  ;[1 1 1] Num
  (`self.Gerer_bouton` self "NewEnumerator0" "2" OtherActor (`self.bouton num 2`) (`self.Move num 2`)))

(event `self.Zone_overlap_num 3.OnComponentBeginOverlap`
  (params (OverlappedComponent :type "PrimitiveComponent Object Reference") (OtherActor :type "Actor Object Reference") (OtherComp :type "PrimitiveComponent Object Reference") (OtherBodyIndex :type Integer) (bFromSweep :type Boolean) (SweepResult :type "HitResult Structure (by ref)"))
  ;[1 1 1] Num
  (`self.Gerer_bouton` self "NewEnumerator0" "3" OtherActor (`self.bouton num 3`) (`self.Move num 3`)))

(event `self.Zone_overlap_num 4.OnComponentBeginOverlap`
  (params (OverlappedComponent :type "PrimitiveComponent Object Reference") (OtherActor :type "Actor Object Reference") (OtherComp :type "PrimitiveComponent Object Reference") (OtherBodyIndex :type Integer) (bFromSweep :type Boolean) (SweepResult :type "HitResult Structure (by ref)"))
  ;[1 1 1] Num
  (`self.Gerer_bouton` self "NewEnumerator0" "4" OtherActor (`self.bouton num 4`) (`self.Move num 4`)))

(event `self.Zone_overlap_num 5.OnComponentBeginOverlap`
  (params (OverlappedComponent :type "PrimitiveComponent Object Reference") (OtherActor :type "Actor Object Reference") (OtherComp :type "PrimitiveComponent Object Reference") (OtherBodyIndex :type Integer) (bFromSweep :type Boolean) (SweepResult :type "HitResult Structure (by ref)"))
  ;[1 1 1] Num
  (`self.Gerer_bouton` self "NewEnumerator0" "5" OtherActor (`self.bouton num 5`) (`self.Move num 5`)))

(event `self.Zone_overlap_num 6.OnComponentBeginOverlap`
  (params (OverlappedComponent :type "PrimitiveComponent Object Reference") (OtherActor :type "Actor Object Reference") (OtherComp :type "PrimitiveComponent Object Reference") (OtherBodyIndex :type Integer) (bFromSweep :type Boolean) (SweepResult :type "HitResult Structure (by ref)"))
  ;[1 1 1] Num
  (`self.Gerer_bouton` self "NewEnumerator0" "6" OtherActor (`self.bouton num 6`) (`self.Move num 6`)))

(event `self.Zone_overlap_num 7.OnComponentBeginOverlap`
  (params (OverlappedComponent :type "PrimitiveComponent Object Reference") (OtherActor :type "Actor Object Reference") (OtherComp :type "PrimitiveComponent Object Reference") (OtherBodyIndex :type Integer) (bFromSweep :type Boolean) (SweepResult :type "HitResult Structure (by ref)"))
  ;[1 1 1] Num
  (`self.Gerer_bouton` self "NewEnumerator0" "7" OtherActor (`self.bouton num 7`) (`self.Move num 7`)))

(event `self.Zone_overlap_num 8.OnComponentBeginOverlap`
  (params (OverlappedComponent :type "PrimitiveComponent Object Reference") (OtherActor :type "Actor Object Reference") (OtherComp :type "PrimitiveComponent Object Reference") (OtherBodyIndex :type Integer) (bFromSweep :type Boolean) (SweepResult :type "HitResult Structure (by ref)"))
  ;[1 1 1] Num
  (`self.Gerer_bouton` self "NewEnumerator0" "8" OtherActor (`self.bouton num 8`) (`self.Move num 8`)))

(event `self.Zone_overlap_num 9.OnComponentBeginOverlap`
  (params (OverlappedComponent :type "PrimitiveComponent Object Reference") (OtherActor :type "Actor Object Reference") (OtherComp :type "PrimitiveComponent Object Reference") (OtherBodyIndex :type Integer) (bFromSweep :type Boolean) (SweepResult :type "HitResult Structure (by ref)"))
  ;[1 1 1] Num
  (`self.Gerer_bouton` self "NewEnumerator0" "9" OtherActor (`self.bouton num 9`) (`self.Move num 9`)))

(event `self.Zone_overlap_dot.OnComponentBeginOverlap`
  (params (OverlappedComponent :type "PrimitiveComponent Object Reference") (OtherActor :type "Actor Object Reference") (OtherComp :type "PrimitiveComponent Object Reference") (OtherBodyIndex :type Integer) (bFromSweep :type Boolean) (SweepResult :type "HitResult Structure (by ref)"))
  ;[1 1 1] Num
  (`self.Gerer_bouton` self "NewEnumerator0" "." OtherActor (`self.bouton dot`) (`self.Move dot`)))

(fn `Define_focus`
  (params (Focus :type Boolean))
  (returns (Ok :type Boolean))
  (return false))

(fn `Gestion bouton`
  (params (Mode :type "/Game/Briques_projets/Clavier/Tablette_bouton_fonction/ENUM_Bouton Enum" :default "NewEnumerator0") (Valeur_bouton :type String))
  (returns (Succes :type Boolean))
  (bind (_parameters_kinect_lmin _parameters_kinect_lmax _parameters_kinect_hmin _parameters_kinect_hmax _parameters_kinect_dmin _parameters_kinect_dmax _parameters_kinect_nbvalmoy _parameters_kinect_simplification) (break `/Game/Briques_projets_rg2/Kinect_webserver/STR_Param_kinect` (`/Game/Briques_projets_rg2/Kinect_webserver/BP_serveur_kinect.Parameters kinect` (`self.Serveur kinect`))))
  (switch `/Game/Briques_projets/Clavier/Tablette_bouton_fonction/ENUM_Bouton` Mode
    (:`NewEnumerator0`
      (if (< (`KismetStringLibrary.Len` Valeur_bouton) 15)
        (bind _output_get (set `self.IP writed` (`KismetStringLibrary.Concat_StrStr` (`self.IP writed`) Valeur_bouton)))
        (`TextRenderComponent.K2_SetText` (`self.IP`) (`KismetTextLibrary.Conv_StringToText` _output_get))
        (return true)))
    (:`NewEnumerator1`
      (`/Game/Briques_projets/Clavier/Tablette_bouton_fonction/BP_Tablette_fonction.Actualise parameters` (`self.BP tablette`) (make `/Game/Briques_projets_rg2/Kinect_webserver/STR_Param_kinect` _parameters_kinect_lmin _parameters_kinect_lmax _parameters_kinect_hmin _parameters_kinect_hmax _parameters_kinect_dmin _parameters_kinect_dmax _parameters_kinect_nbvalmoy _parameters_kinect_simplification (`self.IP writed`)))
      (`self.K2_DestroyActor`)
      (return true))
    (:`NewEnumerator2`
      (bind _output_get_2 (set `self.IP writed` (`KismetStringLibrary.LeftChop` (`self.IP writed`) 1)))
      (`TextRenderComponent.K2_SetText` (`self.IP`) (`KismetTextLibrary.Conv_StringToText` _output_get_2))
      (return true))
    (:`NewEnumerator3`
      (bind _output_get_3 (set `self.IP writed` ""))
      (`TextRenderComponent.K2_SetText` (`self.IP`) (`KismetTextLibrary.Conv_StringToText` _output_get_3))
      (return true))))

(fn `IsHeld`
  (returns (bHeld :type Boolean) (AttachedToParent :type "SceneComponent Object Reference"))
  (return false null))

(fn `UserConstructionScript`)