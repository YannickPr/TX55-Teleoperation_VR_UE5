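; BP_API is an experimental Blueprint for testing HTTP/JSON calls through the VaRest plugin.
; CustomEvent_1 only creates and stores an empty JSON object, while two callbacks print either a whole response or its utc_datetime field.
; The requests that would use those callbacks, a world time GET and a local depth-sensor PUT, are disconnected, as is a JSON decode of a property-read payload.
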(event `CustomEvent_1`
  (bind _returnvalue (`VaRestSubsystem.ConstructVaRestJsonObject` (subsystem `VaRestSubsystem`)))
  (set `self.Json_var` _returnvalue))

(event `CustomEvent5`
  (params (Request :type "VaRestRequestJSON Object Reference"))
  (`KismetSystemLibrary.PrintString` (`VaRestJsonObject.EncodeJson` (`VaRestRequestJSON.GetResponseObject` Request)) true true (struct :`G` 0.66 :`B` 1.0 :`A` 1.0) 20.0))

(event `JsonRequest`
  (params (Request :type "VaRestRequestJSON Object Reference"))
  (`KismetSystemLibrary.PrintString` (`VaRestJsonObject.GetStringField` (`VaRestRequestJSON.GetResponseObject` Request) "utc_datetime")))