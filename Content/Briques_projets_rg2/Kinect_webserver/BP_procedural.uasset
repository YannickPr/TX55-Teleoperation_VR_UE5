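; Procedural mesh Blueprint that turns depth data, apparently from a Kinect, into a surface mesh.
; Generermaillage stores crop, depth range and simplification settings, then launches a multithreaded function projecting in-range samples into a vertex grid using camera FOV angles.
; Grid triangles are kept if beyond 50 cm and not too stretched, with unnormalized normals taken from each cell's first triangle.
; An artificial latency from Parent delays mesh creation, which then clears Parent's LoadingMesh flag.
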(event `Generer maillage`
  (params (Parameters :type "/Game/Briques_projets_rg2/Kinect_webserver/STR_Param_kinect Structure") (Data :type "Array of Integer (by ref)") (Parent :type "/Game/Briques_projets_rg2/Kinect_webserver/BP_serveur_kinect Object Reference"))
  ;[1 1 1] initialisation
  (set `self.De_largeur` Parameters_Lmin_2_ABF6A6FB4196972BE1D82783AB88F8C7)
  (set `self.A_largeur` Parameters_Lmax_6_89373B734E50EC7ECFE2E9BFC4731114)
  (set `self.De_hauteur` Parameters_Hmin_7_C83BDE4E44EF76260EF536ACD589801C)
  (set `self.A_hauteur` Parameters_Hmax_8_BADCDA6A4B3AFA9C1B8870BFBA98E0A9)
  (set `self.De profondeur` (* Parameters_Dmin_11_CAC71ED44E6D24F7D1EAC38186885763 10))
  (set `self.A profondeur` (* Parameters_Dmax_12_2CFCA264413436790BFCAD93D109FC58 10))
  (set `self.Simplification` Parameters_Simplification_17_A19F9FE14DFF9DB1AF9E189D73A67E08)
  (set `self.Data` Data)
  (set `self.Parent` Parent)
  ;[0.4307 0.2384 0.724] Background task
  (`MultithreadedLibrary.CallMultithreadedFunction` self))

(event `self.MultithreadedFunction`
  (bind (_seconds _partialseconds) (`GameplayStatics.GetAccurateRealTime`))
  (bind (_seconds_2 _partialseconds_2) (`GameplayStatics.GetAccurateRealTime`))
  (bind _proceduralmesh (`self.ProceduralMesh`))
  (bind _vertices (`self.Vertices`))
  (bind _position_triangles (`self.Position triangles`))
  (bind _position_triangles_2 (`self.Position triangles`))
  (bind _largeur_selection (`self.Largeur selection`))
  (bind _normals (`self.Normals`))
  (bind _simplification (`self.Simplification`))
  (bind _simplification_2 (`self.Simplification`))
  (bind _returnvalue (* (`self.Largeur selection`) (`self.Hauteur selection`)))
  (bind _returnvalue_2 (+ _position_triangles 1))
  (bind _returnvalue_3 (+ _position_triangles (`self.Largeur selection`)))
  (bind _returnvalue_4 (+ _position_triangles_2 _largeur_selection 1))
  (bind _returnvalue_5 (+ _position_triangles_2 _largeur_selection 0))
  (bind _returnvalue_6 (+ _position_triangles_2 1))
  (bind _returnvalue_7 (/ (- (`self.A_largeur`) (`self.De_largeur`)) _simplification))
  (bind _returnvalue_8 (/ (- (`self.A_hauteur`) (`self.De_hauteur`)) _simplification_2))
  ;[1 1 1] initialize variables
  ;;[0.4307 0.2384 0.724] Background task
  (set `self.Temps init latence` (+ _partialseconds _seconds))
  (`self.Print delta temps` "Start")
  (`KismetArrayLibrary.Array_Clear` (`self.Triangles`))
  ;;[1 0 0.04724] Valeurs impaires non prise en charge
  (set `self.Largeur selection` (+ _returnvalue_7 1))
  (set `self.A_largeur` (+ (`self.De_largeur`) (* _returnvalue_7 _simplification)))
  (set `self.Hauteur selection` (+ _returnvalue_8 1))
  (set `self.A_hauteur` (+ (`self.De_hauteur`) (* _returnvalue_8 _simplification_2)))
  (`KismetArrayLibrary.Array_Clear` _vertices)
  (`KismetArrayLibrary.Array_Resize` _vertices _returnvalue)
  (`KismetArrayLibrary.Array_Clear` _normals)
  (`KismetArrayLibrary.Array_Resize` _normals _returnvalue)
  ;[1 1 1] For each row
  (for _index (range (`self.Hauteur selection`))
    (set `self.Index hauteur` _index)
    ;[1 1 1] For each line
    (for _index_2 (range (`self.Largeur selection`))
      (set `self.Index largeur` _index_2)
      (bind _output_get (set `self.Index local` (+ _index_2 (* (`self.Index hauteur`) (`self.Largeur selection`)))))
      (bind _output (`|GetArrayItem` (`self.Data`) _output_get))
      ;[1 1 1] If valide, create point
      (if (and (> _output (`self.De profondeur`)) (< _output (`self.A profondeur`)))
        (`KismetArrayLibrary.Array_Set` (`self.Vertices`) (`self.Index local`) (`self.Determiner position point` (+ (* (`self.Index largeur`) (`self.Simplification`)) (`self.De_largeur`)) (+ (* (`self.Index hauteur`) (`self.Simplification`)) (`self.De_hauteur`)) (/ (`KismetMathLibrary.Conv_IntToDouble` _output) 10.0)) true))))
  (`self.Print delta temps` "Fin points")
  ;[1 1 1] For each row/line oh triangles
  (set `self.Position triangles` 0)
  (for _ (range (+ (- (`self.Hauteur selection`) 2) 1))
    (for _ (range (+ (- (`self.Largeur selection`) 2) 1))
      ;[1 1 1] Add triangle and normal
      (`|ExecutionSequence`
        (:`then_0`
          (bind _valide__ (`self.IsValidTriangle` _position_triangles _returnvalue_2 _returnvalue_3))
          (if _valide__
            (`self.AddNormal` _position_triangles _returnvalue_2 _returnvalue_3)
            (`KismetArrayLibrary.Array_Append` (`self.Triangles`) (`|MakeArray` _position_triangles _returnvalue_2 _returnvalue_3))))
        (:`then_1`
          (bind _valide___2 (`self.IsValidTriangle` _returnvalue_6 _returnvalue_4 _returnvalue_5))
          (if _valide___2
            (`KismetArrayLibrary.Array_Append` (`self.Triangles`) (`|MakeArray` _returnvalue_6 _returnvalue_4 _returnvalue_5))))
        (:`then_2`
          (`/Engine/EditorBlueprintResources/StandardMacros.IncrementInt` (`self.Position triangles`)))))
    (`/Engine/EditorBlueprintResources/StandardMacros.IncrementInt` (`self.Position triangles`)))
  ;[1 1 1] Artificial latency for experimentation
  (`self.Print delta temps` "fin triangles")
  (if (>= (+ _partialseconds_2 _seconds_2) (+ (`self.Temps init latence`) (`/Game/Briques_projets_rg2/Kinect_webserver/BP_serveur_kinect.Latence` (`self.Parent`)))) :!label _label
    ;[1 1 1] Crete the mesh
    (`ProceduralMeshComponent.ClearAllMeshSections` _proceduralmesh)
    (`ProceduralMeshComponent.CreateMeshSection_LinearColor` :`self` _proceduralmesh :`Vertices` (`self.Vertices`) :`Triangles` (`self.Triangles`) :`Normals` (`self.Normals`))
    (`PrimitiveComponent.SetMaterial` _proceduralmesh 0 "/Game/Briques_projets_rg2/Kinect_webserver/MA_maillage.MA_maillage")
    (set `/Game/Briques_projets_rg2/Kinect_webserver/BP_serveur_kinect.Loading mesh` false (`self.Parent`))
    (else
      (`KismetSystemLibrary.Delay` 0.05)
      (goto _label))))

(fn `AddNormal`
  (params (`Position P1` :type "Integer (by ref)") (`Position P2` :type "Integer (by ref)") (`Position P3` :type "Integer (by ref)"))
  (bind _vertices (`self.Vertices`))
  (bind _normals (`self.Normals`))
  (bind _output (`|GetArrayItem` _vertices `Position P2`))
  (bind _returnvalue (`KismetMathLibrary.Cross_VectorVector` (- (`|GetArrayItem` _vertices `Position P1`) _output) (- (`|GetArrayItem` _vertices `Position P3`) _output)))
  (`KismetArrayLibrary.Array_Set` _normals `Position P1` _returnvalue true)
  (`KismetArrayLibrary.Array_Set` _normals `Position P2` _returnvalue true)
  (`KismetArrayLibrary.Array_Set` _normals `Position P3` _returnvalue true)
  (return))

(fn `Determiner position point`
  (params (`Index largeur` :type "Integer (by ref)") (`Index hauteur` :type "Integer (by ref)") (Distance :type "Float (double-precision) (by ref)"))
  (returns (`position point` :type "Vector Structure"))
  (return (`KismetMathLibrary.MakeVector` Distance (* Distance (`KismetMathLibrary.DegTan` (* (- (/ (`self.Largeur image`) 2) `Index largeur`) (/ (`self.FOV largeur`) (`self.Largeur image`))))) (* Distance (`KismetMathLibrary.DegTan` (* (- (/ (`self.Hauteur image`) 2) `Index hauteur`) (/ (`self.FOV hauteur`) (`self.Hauteur image`))))))))

(fn `IsValidTriangle`
  (params (`Position P1` :type "Integer (by ref)") (`Position P2` :type "Integer (by ref)") (`Position P3` :type "Integer (by ref)"))
  (returns (`Valide ?` :type Boolean))
  (bind _vertices (`self.Vertices`))
  (bind _output (`|GetArrayItem` _vertices `Position P1`))
  (bind _output_2 (`|GetArrayItem` _vertices `Position P2`))
  (bind _output_3 (`|GetArrayItem` _vertices `Position P3`))
  (bind _returnvalue (`KismetMathLibrary.VSizeSquared` (- _output_2 _output_3)))
  (bind _returnvalue_2 (`KismetMathLibrary.VSizeSquared` (- _output _output_2)))
  (bind _returnvalue_3 (`KismetMathLibrary.VSizeSquared` (- _output _output_3)))
  (set `self.IsValide` false)
  ;[1 1 1] Distance min = 50cm (from camera's datasheet)
  (if (> (.x _output) 50.0)
    (if (> (.x _output_2) 50.0)
      (if (> (.x _output_3) 50.0)
        ;[1 1 1] Is triangle proportion ok ? or at least about ok...
        (if (< (`KismetMathLibrary.FMax` _returnvalue_2 _returnvalue_3 _returnvalue) (* (`KismetMathLibrary.FMin` _returnvalue_2 _returnvalue_3 _returnvalue) 12.0))
          (set `self.IsValide` true)))))
  (return (`self.IsValide`)))

(fn `Print delta temps`
  (params (message :type String))
  (bind (_seconds _partialseconds) (`GameplayStatics.GetAccurateRealTime`))
  (set `self.Temps init` (+ _partialseconds _seconds)))

(fn `UserConstructionScript`)