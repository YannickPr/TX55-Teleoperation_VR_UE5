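; Kinect capture-zone editor actor, owned by BP_Tablette_fonction, showing the sensor's crop volume with draggable handles.
; On BeginPlay it converts the owner's pixel bounds to angles and spawns six attached BP_handle_v2 handles for horizontal, vertical and depth limits.
; Handle moves are projected and clamped, then pushed back through ActualiseParameters.
; SetMesh rebuilds a procedural truncated-pyramid mesh to display the volume; destruction removes the handles.
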(event `self.ReceiveBeginPlay`
  (bind _l_min__d_ (`self.L min (D)`))
  (bind _l_max__d_ (`self.L max (D)`))
  (bind _h_min__d_ (`self.H min (D)`))
  (bind _h_max__d_ (`self.H max (D)`))
  (bind _largeur__pt_ (`self.Largeur (pt)`))
  (bind _hauteur__pt_ (`self.Hauteur (pt)`))
  (bind _returnvalue (/ _largeur__pt_ 2))
  (bind _returnvalue_2 (/ (`self.Largeur (D)`) _largeur__pt_))
  (bind _returnvalue_3 (/ _hauteur__pt_ 2))
  (bind _returnvalue_4 (/ (`self.Hauteur (D)`) _hauteur__pt_))
  (bind _asbp_tablette_fonction (cast `/Game/Briques_projets/Clavier/Tablette_bouton_fonction/BP_Tablette_fonction` (`self.GetOwner` self))
    (:`then`
      (set `self.As BP Tablette Fonction` _asbp_tablette_fonction)
      (bind (_param_kinect_lmin _param_kinect_lmax _param_kinect_hmin _param_kinect_hmax _param_kinect_dmin _param_kinect_dmax) (break `/Game/Briques_projets_rg2/Kinect_webserver/STR_Param_kinect` (`/Game/Briques_projets/Clavier/Tablette_bouton_fonction/BP_Tablette_fonction.Param kinect` _asbp_tablette_fonction)))
      (set `self.L min (D)` (* (- _param_kinect_lmin _returnvalue) _returnvalue_2))
      (set `self.L max (D)` (* (- _param_kinect_lmax _returnvalue) _returnvalue_2))
      (set `self.H min (D)` (* (- _param_kinect_hmin _returnvalue_3) _returnvalue_4))
      (set `self.H max (D)` (* (- _param_kinect_hmax _returnvalue_3) _returnvalue_4))
      (set `self.D min` (`KismetMathLibrary.Conv_IntToDouble` _param_kinect_dmin))
      (set `self.D max` (`KismetMathLibrary.Conv_IntToDouble` _param_kinect_dmax))
      ;[1 1 1] Spawn handles and initialize then with correct position
      (for _index (range 6)
        (bind _returnvalue_5 (`|SpawnActorFromClass` "/Game/Briques_projets/Grab/Handle_v2/BP_handle_v2.BP_handle_v2_C" (`KismetMathLibrary.MakeTransform` (select `int` _index :`0` (`KismetMathLibrary.MakeVector` (* (`self.Distance handle`) (`KismetMathLibrary.DegCos` _l_min__d_)) (* (`self.Distance handle`) (`KismetMathLibrary.DegSin` _l_min__d_))) :`1` (`KismetMathLibrary.MakeVector` (* (`self.Distance handle`) (`KismetMathLibrary.DegCos` _l_max__d_)) (* (`self.Distance handle`) (`KismetMathLibrary.DegSin` _l_max__d_))) :`2` (`KismetMathLibrary.MakeVector` (* (`self.Distance handle`) (`KismetMathLibrary.DegCos` _h_min__d_)) 0.0 (* (`self.Distance handle`) (`KismetMathLibrary.DegSin` _h_min__d_))) :`3` (`KismetMathLibrary.MakeVector` (* (`self.Distance handle`) (`KismetMathLibrary.DegCos` _h_max__d_)) 0.0 (* (`self.Distance handle`) (`KismetMathLibrary.DegSin` _h_max__d_))) :`4` (`KismetMathLibrary.MakeVector` (+ (/ (`self.D min`) 10.0) 5.0)) :`5` (`KismetMathLibrary.MakeVector` (+ (/ (`self.D max`) 10.0) 5.0)))) "AlwaysSpawn" "OverrideRootScale" self null))
        (`self.K2_AttachToActor` _returnvalue_5 self "None" "KeepRelative" "KeepRelative" "KeepRelative" true)
        (`/Game/Briques_projets/Grab/Handle_v2/BP_handle_v2.Initialisation` _returnvalue_5 null null (`KismetMathLibrary.MakeTransform` (0.0 0.0 0.0) (struct) (0.015 0.015 0.015)) self)
        (`KismetArrayLibrary.Array_Add` (`self.Handles`) _returnvalue_5)
        (`self.Set mesh`)))
    (:`CastFailed`
      (`KismetSystemLibrary.PrintString` "Erreur le propriétaire n'est pas le bp tablette fonction"))))

(event `self.ReceiveDestroyed`
  (`KismetSystemLibrary.PrintString` "BP zoom kinect : destroyed, suppression des poignées")
  (for _array_element (`self.Handles`)
    (`self.K2_DestroyActor` _array_element)))

(fn `Communicate_data_handle`
  (params (Position :type "Vector Structure") (Rotation :type "Rotator Structure") (`Ref handle` :type "/Game/Briques_projets/Grab/Handle_v2/BP_handle_v2 Object Reference") (`Object to move` :type "Actor Object Reference"))
  (returns (`Controlled by target` :type Boolean))
  (locals (`_Object to move` :type "Actor Object Reference"))
  (bind _as_bp_tablette_fonction (`self.As BP Tablette Fonction`))
  (bind _defaultsceneroot (`self.DefaultSceneRoot`))
  (bind _defaultsceneroot_2 (`self.DefaultSceneRoot`))
  (bind _defaultsceneroot_3 (`self.DefaultSceneRoot`))
  (bind _defaultsceneroot_4 (`self.DefaultSceneRoot`))
  (bind _as_bp_tablette_fonction_2 (`self.As BP Tablette Fonction`))
  (bind _defaultsceneroot_5 (`self.DefaultSceneRoot`))
  (bind _largeur__pt_ (`self.Largeur (pt)`))
  (bind _largeur__pt__2 (`self.Largeur (pt)`))
  (bind _hauteur__pt_ (`self.Hauteur (pt)`))
  (bind _hauteur__pt__2 (`self.Hauteur (pt)`))
  (bind _as_bp_tablette_fonction_3 (`self.As BP Tablette Fonction`))
  (bind _defaultsceneroot_6 (`self.DefaultSceneRoot`))
  (bind _as_bp_tablette_fonction_4 (`self.As BP Tablette Fonction`))
  (bind _as_bp_tablette_fonction_5 (`self.As BP Tablette Fonction`))
  (bind _as_bp_tablette_fonction_6 (`self.As BP Tablette Fonction`))
  (bind (_param_kinect_lmin _param_kinect_lmax _param_kinect_hmin _param_kinect_hmax _param_kinect_dmin _param_kinect_dmax _param_kinect_nbvalmoy _param_kinect_simplification _param_kinect_ip) (break `/Game/Briques_projets_rg2/Kinect_webserver/STR_Param_kinect` (`/Game/Briques_projets/Clavier/Tablette_bouton_fonction/BP_Tablette_fonction.Param kinect` _as_bp_tablette_fonction)))
  (bind (_param_kinect_lmin_2 _param_kinect_lmax_2 _param_kinect_hmin_2 _param_kinect_hmax_2 _param_kinect_dmin_2 _param_kinect_dmax_2 _param_kinect_nbvalmoy_2 _param_kinect_simplification_2 _param_kinect_ip_2) (break `/Game/Briques_projets_rg2/Kinect_webserver/STR_Param_kinect` (`/Game/Briques_projets/Clavier/Tablette_bouton_fonction/BP_Tablette_fonction.Param kinect` _as_bp_tablette_fonction_2)))
  (bind (_param_kinect_lmin_3 _param_kinect_lmax_3 _param_kinect_hmin_3 _param_kinect_hmax_3 _param_kinect_dmin_3 _param_kinect_dmax_3 _param_kinect_nbvalmoy_3 _param_kinect_simplification_3 _param_kinect_ip_3) (break `/Game/Briques_projets_rg2/Kinect_webserver/STR_Param_kinect` (`/Game/Briques_projets/Clavier/Tablette_bouton_fonction/BP_Tablette_fonction.Param kinect` _as_bp_tablette_fonction_3)))
  (bind (_param_kinect_lmin_4 _param_kinect_lmax_4 _param_kinect_hmin_4 _param_kinect_hmax_4 _param_kinect_dmin_4 _param_kinect_dmax_4 _param_kinect_nbvalmoy_4 _param_kinect_simplification_4 _param_kinect_ip_4) (break `/Game/Briques_projets_rg2/Kinect_webserver/STR_Param_kinect` (`/Game/Briques_projets/Clavier/Tablette_bouton_fonction/BP_Tablette_fonction.Param kinect` _as_bp_tablette_fonction_4)))
  (bind (_param_kinect_lmin_5 _param_kinect_lmax_5 _param_kinect_hmin_5 _param_kinect_hmax_5 _param_kinect_dmin_5 _param_kinect_dmax_5 _param_kinect_nbvalmoy_5 _param_kinect_simplification_5 _param_kinect_ip_5) (break `/Game/Briques_projets_rg2/Kinect_webserver/STR_Param_kinect` (`/Game/Briques_projets/Clavier/Tablette_bouton_fonction/BP_Tablette_fonction.Param kinect` _as_bp_tablette_fonction_5)))
  (bind (_param_kinect_lmin_6 _param_kinect_lmax_6 _param_kinect_hmin_6 _param_kinect_hmax_6 _param_kinect_dmin_6 _param_kinect_dmax_6 _param_kinect_nbvalmoy_6 _param_kinect_simplification_6 _param_kinect_ip_6) (break `/Game/Briques_projets_rg2/Kinect_webserver/STR_Param_kinect` (`/Game/Briques_projets/Clavier/Tablette_bouton_fonction/BP_Tablette_fonction.Param kinect` _as_bp_tablette_fonction_6)))
  (bind _returnvalue (`KismetMathLibrary.ProjectVectorOnToPlane` (- Position (`SceneComponent.K2_GetComponentLocation` (`self.DefaultSceneRoot`))) (`SceneComponent.GetUpVector` _defaultsceneroot)))
  (bind _returnvalue_2 (`KismetMathLibrary.ProjectVectorOnToPlane` (- Position (`SceneComponent.K2_GetComponentLocation` (`self.DefaultSceneRoot`))) (`SceneComponent.GetRightVector` _defaultsceneroot_5)))
  (bind _returnvalue_3 (* (- (`KismetMathLibrary.VSize` (`KismetMathLibrary.ProjectVectorOnToVector` (- Position (`SceneComponent.K2_GetComponentLocation` (`self.DefaultSceneRoot`))) (`SceneComponent.GetForwardVector` (`self.DefaultSceneRoot`)))) 5.0) 10.0))
  (bind _returnvalue_4 (* (`KismetMathLibrary.DegAcos` (/ (`KismetMathLibrary.Dot_VectorVector` _returnvalue_2 (`SceneComponent.GetForwardVector` _defaultsceneroot_5)) (`KismetMathLibrary.VSize` _returnvalue_2))) (`KismetMathLibrary.SelectFloat` 1.0 -1.0 (> (`KismetMathLibrary.Dot_VectorVector` _returnvalue_2 (`SceneComponent.GetUpVector` _defaultsceneroot_5)) 0.0))))
  (bind _returnvalue_5 (* (`KismetMathLibrary.DegAcos` (/ (`KismetMathLibrary.Dot_VectorVector` _returnvalue (`SceneComponent.GetForwardVector` _defaultsceneroot)) (`KismetMathLibrary.VSize` _returnvalue))) (`KismetMathLibrary.SelectFloat` 1.0 -1.0 (> (`KismetMathLibrary.Dot_VectorVector` _returnvalue (`SceneComponent.GetRightVector` _defaultsceneroot)) 0.0))))
  (set `local._Object to move` `Object to move`)
  (switch `int` (`KismetArrayLibrary.Array_Find` (`self.Handles`) `Ref handle`)
    (:`0`
      ;[1 1 1] L min
      (bind _output_get (set `self.L min (D)` (`KismetMathLibrary.FClamp` _returnvalue_5 (/ (`self.Largeur (D)`) -2.0) (- (`self.L max (D)`) 5.0))))
      (`/Game/Briques_projets/Clavier/Tablette_bouton_fonction/BP_Tablette_fonction.Actualise parameters` _as_bp_tablette_fonction_3 (make `/Game/Briques_projets_rg2/Kinect_webserver/STR_Param_kinect` (`KismetMathLibrary.Clamp` (+ (/ _largeur__pt_ 2) (`KismetMathLibrary.FTrunc` (* _output_get (/ _largeur__pt_ (`self.Largeur (D)`))))) 0 511) _param_kinect_lmax_3 _param_kinect_hmin_3 _param_kinect_hmax_3 _param_kinect_dmin_3 _param_kinect_dmax_3 _param_kinect_nbvalmoy_3 _param_kinect_simplification_3 _param_kinect_ip_3))
      (`self.Set mesh`)
      (`self.K2_SetActorLocation` (`local._Object to move`) (+ (* (`self.Distance handle`) (`KismetMathLibrary.DegCos` _output_get) (`SceneComponent.GetForwardVector` _defaultsceneroot_2)) (* (`self.Distance handle`) (`KismetMathLibrary.DegSin` _output_get) (`SceneComponent.GetRightVector` _defaultsceneroot_2)) (`SceneComponent.K2_GetComponentLocation` (`self.DefaultSceneRoot`))) false false)
      (return true))
    (:`1`
      ;[1 1 1] L max
      (bind _output_get_2 (set `self.L max (D)` (`KismetMathLibrary.FClamp` _returnvalue_5 (+ (`self.L min (D)`) 5.0) (/ (`self.Largeur (D)`) 2.0))))
      (`/Game/Briques_projets/Clavier/Tablette_bouton_fonction/BP_Tablette_fonction.Actualise parameters` _as_bp_tablette_fonction (make `/Game/Briques_projets_rg2/Kinect_webserver/STR_Param_kinect` _param_kinect_lmin (`KismetMathLibrary.Clamp` (+ (/ _largeur__pt__2 2) (`KismetMathLibrary.FTrunc` (* _output_get_2 (/ _largeur__pt__2 (`self.Largeur (D)`))))) 0 511) _param_kinect_hmin _param_kinect_hmax _param_kinect_dmin _param_kinect_dmax _param_kinect_nbvalmoy _param_kinect_simplification _param_kinect_ip))
      (`self.Set mesh`)
      (`self.K2_SetActorLocation` (`local._Object to move`) (+ (* (* (`self.Distance handle`) (`KismetMathLibrary.DegCos` _output_get_2)) (`SceneComponent.GetForwardVector` _defaultsceneroot_3)) (* (* (`self.Distance handle`) (`KismetMathLibrary.DegSin` _output_get_2)) (`SceneComponent.GetRightVector` _defaultsceneroot_3)) (`SceneComponent.K2_GetComponentLocation` (`self.DefaultSceneRoot`))) false false)
      (return true))
    (:`2`
      ;[1 1 1] H min
      (bind _output_get_3 (set `self.H min (D)` (`KismetMathLibrary.FClamp` _returnvalue_4 (/ (`self.Hauteur (D)`) -2.0) (- (`self.H max (D)`) 5.0))))
      (`/Game/Briques_projets/Clavier/Tablette_bouton_fonction/BP_Tablette_fonction.Actualise parameters` _as_bp_tablette_fonction_4 (make `/Game/Briques_projets_rg2/Kinect_webserver/STR_Param_kinect` _param_kinect_lmin_4 _param_kinect_lmax_4 (`KismetMathLibrary.Clamp` (+ (/ _hauteur__pt__2 2) (`KismetMathLibrary.FTrunc` (* _output_get_3 (/ _hauteur__pt__2 (`self.Hauteur (D)`))))) 0 423) _param_kinect_hmax_4 _param_kinect_dmin_4 _param_kinect_dmax_4 _param_kinect_nbvalmoy_4 _param_kinect_simplification_4 _param_kinect_ip_4))
      (`self.Set mesh`)
      (`self.K2_SetActorLocation` (`local._Object to move`) (+ (* (* (`self.Distance handle`) (`KismetMathLibrary.DegCos` _output_get_3)) (`SceneComponent.GetForwardVector` _defaultsceneroot_4)) (* (* (`self.Distance handle`) (`KismetMathLibrary.DegSin` _output_get_3)) (`SceneComponent.GetUpVector` _defaultsceneroot_4)) (`SceneComponent.K2_GetComponentLocation` (`self.DefaultSceneRoot`))) false false)
      (return true))
    (:`3`
      ;[1 1 1] H max
      (bind _output_get_4 (set `self.H max (D)` (`KismetMathLibrary.FClamp` _returnvalue_4 (+ (`self.H min (D)`) 5.0) (/ (`self.Hauteur (D)`) 2.0))))
      (`/Game/Briques_projets/Clavier/Tablette_bouton_fonction/BP_Tablette_fonction.Actualise parameters` _as_bp_tablette_fonction_5 (make `/Game/Briques_projets_rg2/Kinect_webserver/STR_Param_kinect` _param_kinect_lmin_5 _param_kinect_lmax_5 _param_kinect_hmin_5 (`KismetMathLibrary.Clamp` (+ (/ _hauteur__pt_ 2) (`KismetMathLibrary.FTrunc` (* _output_get_4 (/ _hauteur__pt_ (`self.Hauteur (D)`))))) 0 423) _param_kinect_dmin_5 _param_kinect_dmax_5 _param_kinect_nbvalmoy_5 _param_kinect_simplification_5 _param_kinect_ip_5))
      (`self.Set mesh`)
      (`self.K2_SetActorLocation` (`local._Object to move`) (+ (* (* (`self.Distance handle`) (`KismetMathLibrary.DegCos` _output_get_4)) (`SceneComponent.GetForwardVector` _defaultsceneroot_6)) (* (* (`self.Distance handle`) (`KismetMathLibrary.DegSin` _output_get_4)) (`SceneComponent.GetUpVector` _defaultsceneroot_6)) (`SceneComponent.K2_GetComponentLocation` (`self.DefaultSceneRoot`))) false false)
      (return true))
    (:`4`
      ;[1 1 1] D min
      (bind _output_get_5 (set `self.D min` (`KismetMathLibrary.FClamp` _returnvalue_3 50.0 (- (`self.D max`) 10.0))))
      (`/Game/Briques_projets/Clavier/Tablette_bouton_fonction/BP_Tablette_fonction.Actualise parameters` _as_bp_tablette_fonction_6 (make `/Game/Briques_projets_rg2/Kinect_webserver/STR_Param_kinect` _param_kinect_lmin_6 _param_kinect_lmax_6 _param_kinect_hmin_6 _param_kinect_hmax_6 (`KismetMathLibrary.FTrunc` _output_get_5) _param_kinect_dmax_6 _param_kinect_nbvalmoy_6 _param_kinect_simplification_6 _param_kinect_ip_6))
      (`self.Set mesh`)
      (`self.K2_SetActorLocation` (`local._Object to move`) (+ (* (+ (/ _output_get_5 10.0) 5.0) (`SceneComponent.GetForwardVector` (`self.DefaultSceneRoot`))) (`SceneComponent.K2_GetComponentLocation` (`self.DefaultSceneRoot`))) false false)
      (return true))
    (:`5`
      ;[1 1 1] D max
      (bind _output_get_6 (set `self.D max` (`KismetMathLibrary.FClamp` _returnvalue_3 (+ (`self.D min`) 10.0) 600.0)))
      (`/Game/Briques_projets/Clavier/Tablette_bouton_fonction/BP_Tablette_fonction.Actualise parameters` _as_bp_tablette_fonction_2 (make `/Game/Briques_projets_rg2/Kinect_webserver/STR_Param_kinect` _param_kinect_lmin_2 _param_kinect_lmax_2 _param_kinect_hmin_2 _param_kinect_hmax_2 _param_kinect_dmin_2 (`KismetMathLibrary.FTrunc` _output_get_6) _param_kinect_nbvalmoy_2 _param_kinect_simplification_2 _param_kinect_ip_2))
      (`self.Set mesh`)
      (`self.K2_SetActorLocation` (`local._Object to move`) (+ (* (+ (/ _output_get_6 10.0) 5.0) (`SceneComponent.GetForwardVector` (`self.DefaultSceneRoot`))) (`SceneComponent.K2_GetComponentLocation` (`self.DefaultSceneRoot`))) false false)
      (return true))))

(fn `Get_handle_details`
  (returns (`Is grabbable` :type Boolean) (`Is Grabbed` :type Boolean))
  (return false false))

(fn `Set mesh`
  (bind _d_min (`self.D min`))
  (bind _d_max (`self.D max`))
  (bind _proceduralmesh (`self.ProceduralMesh`))
  (bind _returnvalue (`KismetMathLibrary.DegTan` (- 0.0 (`self.L max (D)`))))
  (bind _returnvalue_2 (`KismetMathLibrary.DegTan` (- 0.0 (`self.H max (D)`))))
  (bind _returnvalue_3 (`KismetMathLibrary.DegTan` (- 0.0 (`self.H min (D)`))))
  (bind _returnvalue_4 (`KismetMathLibrary.DegTan` (- 0.0 (`self.L min (D)`))))
  (bind _returnvalue_5 (`KismetMathLibrary.DegTan` (- 0.0 (`self.L max (D)`))))
  (bind _returnvalue_6 (`KismetMathLibrary.DegTan` (- 0.0 (`self.H max (D)`))))
  (bind _returnvalue_7 (`KismetMathLibrary.DegTan` (- 0.0 (`self.H min (D)`))))
  (bind _returnvalue_8 (`KismetMathLibrary.DegTan` (- 0.0 (`self.L min (D)`))))
  (bind _returnvalue_9 (/ (+ _returnvalue_2 _returnvalue_3) 2.0))
  (bind _returnvalue_10 (/ (+ _returnvalue_8 _returnvalue) 2.0))
  ;[1 1 1] v2 : pyramide tronquée
  (`KismetSystemLibrary.PrintString` (`KismetStringLibrary.Concat_StrStr` ""))
  (`ProceduralMeshComponent.CreateMeshSection_LinearColor` :`self` _proceduralmesh :`Vertices` (`|MakeArray` (* (`KismetMathLibrary.MakeVector` 1.0 _returnvalue_4 _returnvalue_7) _d_min) (* (`KismetMathLibrary.MakeVector` 1.0 _returnvalue_4 _returnvalue_6) _d_min) (* (`KismetMathLibrary.MakeVector` 1.0 _returnvalue_5 _returnvalue_6) _d_min) (* (`KismetMathLibrary.MakeVector` 1.0 _returnvalue_5 _returnvalue_7) _d_min) (* (`KismetMathLibrary.MakeVector` 1.0 _returnvalue_8 _returnvalue_3) _d_max) (* (`KismetMathLibrary.MakeVector` 1.0 _returnvalue_8 _returnvalue_9) _d_max) (* (`KismetMathLibrary.MakeVector` 1.0 _returnvalue_8 _returnvalue_2) _d_max) (* (`KismetMathLibrary.MakeVector` 1.0 _returnvalue_10 _returnvalue_2) _d_max) (* (`KismetMathLibrary.MakeVector` 1.0 _returnvalue _returnvalue_2) _d_max) (* (`KismetMathLibrary.MakeVector` 1.0 _returnvalue _returnvalue_9) _d_max) (* (`KismetMathLibrary.MakeVector` 1.0 _returnvalue _returnvalue_3) _d_max) (* (`KismetMathLibrary.MakeVector` 1.0 _returnvalue_10 _returnvalue_3) _d_max)) :`Triangles` (`|MakeArray` 0 4 5 0 5 1 1 5 6 1 6 7 1 7 2 2 7 8 2 8 9 2 9 3 3 9 10 3 10 11 3 11 0 0 11 4 0 1 2 0 2 3 4 6 8 4 8 10))
  (`PrimitiveComponent.SetMaterial` _proceduralmesh 0 "/Game/Briques_projets_rg2/Tablette_menu/MA_Zoom_kinect.MA_Zoom_kinect"))

(fn `Use_handle`
  (params (Grabbed :type Boolean) (`Is selected` :type Boolean) (`Grabed by` :type "StaticMeshComponent Object Reference"))
  (returns (`Object to move` :type "Actor Object Reference") (`Handle's target` :type "Actor Object Reference"))
  (return null null))

(fn `UserConstructionScript`)