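; Ghost version of a robot arm that poses its joints to follow a handle position.
; The construction script derives both segment lengths from pivot spacing and scales reach limits and handle offset with the root.
; CommunicateDataHandle yaws the base and its counter-rotating gear toward the handle within angle limits.
; It then clamps the offset target to the reach range and solves arm angles analytically with law-of-cosines inverse kinematics.
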(fn `Communicate_data_handle`
  (params (Position :type "Vector Structure") (Rotation :type "Rotator Structure") (`Ref handle` :type "/Game/Briques_projets/Grab/Handle_v2/BP_handle_v2 Object Reference") (`Object to move` :type "Actor Object Reference"))
  (returns (`Controlled by target` :type Boolean))
  (locals (X :type "Float (double-precision)" :default 0.0))
  (bind (_offset_handle_scaled_x _offset_handle_scaled_y _offset_handle_scaled_z) (`KismetMathLibrary.BreakVector` (`self.Offset handle scaled`)))
  (bind _bati (`self.Bati`))
  (bind _longueur_segment_2 (`self.Longueur segment 2`))
  (bind _longueur_segment_1 (`self.Longueur segment 1`))
  (bind _longueur_segment_1_2 (`self.Longueur segment 1`))
  (bind _returnvalue (`KismetMathLibrary.ProjectVectorOnToPlane` (- (`self.Position handle`) (`SceneComponent.K2_GetComponentLocation` (`self.Bati`))) (`SceneComponent.GetUpVector` (`self.Bati`))))
  (bind (_returnvalue_x _returnvalue_y) (`KismetMathLibrary.BreakVector` (`KismetMathLibrary.Normal` (`KismetMathLibrary.ProjectVectorOnToPlane` (- (`self.Position handle`) (`SceneComponent.K2_GetComponentLocation` (`self.Bati`))) (`KismetMathLibrary.GetUpVector` (`SceneComponent.K2_GetComponentRotation` (`self.Bati`)))) 0.001)))
  (bind _returnvalue_2 (- (- (`self.Position handle`) (`SceneComponent.K2_GetComponentLocation` (`self.Ry_1`))) (`KismetMathLibrary.MakeVector` (* _offset_handle_scaled_x _returnvalue_x) (* _offset_handle_scaled_x _returnvalue_y) _offset_handle_scaled_z)))
  (bind _returnvalue_3 (`KismetMathLibrary.VSize` _returnvalue_2))
  (bind _returnvalue_4 (/ (`self.Atteinte min robot`) _returnvalue_3))
  (bind _returnvalue_5 (/ (`self.Atteinte max robot`) _returnvalue_3))
  (bind _returnvalue_6 (`KismetMathLibrary.SelectVector` (* _returnvalue_2 (`KismetMathLibrary.MakeVector` _returnvalue_4 _returnvalue_4 _returnvalue_4)) (`KismetMathLibrary.SelectVector` (* _returnvalue_2 (`KismetMathLibrary.MakeVector` _returnvalue_5 _returnvalue_5 _returnvalue_5)) _returnvalue_2 (> _returnvalue_3 (`self.Atteinte max robot`))) (< _returnvalue_3 (`self.Atteinte min robot`))))
  (bind _returnvalue_7 (`KismetMathLibrary.VSize` _returnvalue_6))
  (bind _returnvalue_8 (`KismetMathLibrary.ClampAngle` (- 0.0 (`KismetMathLibrary.DegAsin` (/ (`KismetMathLibrary.Dot_VectorVector` _returnvalue_6 (`SceneComponent.GetUpVector` (`self.Bati`))) (`KismetMathLibrary.VSize` _returnvalue_6))) (`KismetMathLibrary.DegAcos` (/ (- (`KismetMathLibrary.Square` (`self.Longueur segment 2`)) (`KismetMathLibrary.Square` _returnvalue_7) (`KismetMathLibrary.Square` _longueur_segment_1_2)) (* _returnvalue_7 _longueur_segment_1_2 -2.0)))) 223.0 345.0))
  (bind _returnvalue_9 (`KismetMathLibrary.FClamp` (`KismetMathLibrary.DegAcos` (/ (- (`KismetMathLibrary.Square` (`KismetMathLibrary.VSize` _returnvalue_6)) (`KismetMathLibrary.Square` _longueur_segment_1) (`KismetMathLibrary.Square` _longueur_segment_2)) (* _longueur_segment_1 _longueur_segment_2 2.0))) (`KismetMathLibrary.FMax` (- 0.0 _returnvalue_8 23.0) 40.0) (`KismetMathLibrary.FMin` (- 0.0 _returnvalue_8 -90.0) 140.0)))
  (bind _returnvalue_10 (+ _returnvalue_8 _returnvalue_9))
  (set `self.Position handle` Position)
  (bind _output_get (set `self.Current Rz` (`KismetMathLibrary.FClamp` (* (`KismetMathLibrary.DegAcos` (/ (`KismetMathLibrary.Dot_VectorVector` _returnvalue (`SceneComponent.GetForwardVector` _bati)) (`KismetMathLibrary.VSize` _returnvalue))) (`KismetMathLibrary.SelectFloat` 1.0 -1.0 (> (`KismetMathLibrary.Dot_VectorVector` _returnvalue (`SceneComponent.GetRightVector` _bati)) 0.0))) -90.0 90.0)))
  (`SceneComponent.K2_SetRelativeRotation` (`self.Rz`) (`KismetMathLibrary.MakeRotator` 0.0 0.0 _output_get) false false)
  (`SceneComponent.K2_SetRelativeRotation` (`self.Rz_pignon`) (`KismetMathLibrary.MakeRotator` 0.0 0.0 (* _output_get -3.5555)) false false)
  (set `self.Current Ry_1` (+ _returnvalue_8 180.0))
  (`SceneComponent.K2_SetRelativeRotation` (`self.Ry_1`) (`KismetMathLibrary.MakeRotator` 0.0 0.0 _returnvalue_8) false false)
  (`SceneComponent.K2_SetRelativeRotation` (`self.Ry_1-2`) (`KismetMathLibrary.MakeRotator` 0.0 0.0 _returnvalue_8) false false)
  (`SceneComponent.K2_SetRelativeRotation` (`self.Ry_2-2`) (`KismetMathLibrary.MakeRotator` 0.0 0.0 (- 0.0 _returnvalue_8)) false false)
  (`SceneComponent.K2_SetRelativeRotation` (`self.Ry_2`) (`KismetMathLibrary.MakeRotator` 0.0 0.0 _returnvalue_9) false false)
  (set `self.Current Ry_2` _returnvalue_10)
  (`SceneComponent.K2_SetRelativeRotation` (`self.Ry_1-3`) (`KismetMathLibrary.MakeRotator` 0.0 0.0 _returnvalue_10) false false)
  (`SceneComponent.K2_SetRelativeRotation` (`self.Ry_1-4`) (`KismetMathLibrary.MakeRotator` 0.0 0.0 (- 0.0 _returnvalue_9)) false false)
  (`SceneComponent.K2_SetRelativeRotation` (`self.Ry_2-3`) (`KismetMathLibrary.MakeRotator` 0.0 0.0 (+ _returnvalue_8 _returnvalue_9)) false false)
  (`SceneComponent.K2_SetRelativeRotation` (`self.R_pignon_1`) (`KismetMathLibrary.MakeRotator` 0.0 0.0 (* _returnvalue_8 -3.5555)) false false)
  (`SceneComponent.K2_SetRelativeRotation` (`self.R_pignon_2`) (`KismetMathLibrary.MakeRotator` 0.0 0.0 (* (+ _returnvalue_8 _returnvalue_9) -3.5555)) false false)
  (`SceneComponent.K2_SetRelativeRotation` (`self.Ry_3`) (`KismetMathLibrary.MakeRotator` 0.0 0.0 (- 0.0 _returnvalue_8 _returnvalue_9)) false false)
  (return false))

(fn `Define_focus`
  (params (Focus :type Boolean))
  (returns (Ok :type Boolean))
  (return false))

(fn `Get_handle_details`
  (returns (`Is grabbable` :type Boolean) (`Is Grabbed` :type Boolean))
  (return false false))

(fn `IsHeld`
  (returns (bHeld :type Boolean) (AttachedToParent :type "SceneComponent Object Reference"))
  (return false null))

(fn `Use_handle`
  (params (Grabbed :type Boolean) (`Is selected` :type Boolean) (`Grabed by` :type "StaticMeshComponent Object Reference"))
  (returns (`Object to move` :type "Actor Object Reference") (`Handle's target` :type "Actor Object Reference"))
  (return null null))

(fn `UserConstructionScript`
  (bind _returnvalue_x (`KismetMathLibrary.BreakVector` (`SceneComponent.K2_GetComponentScale` (`self.DefaultSceneRoot`))))
  (bind _returnvalue (`SceneComponent.K2_GetComponentLocation` (`self.Ry_2`)))
  (set `self.Longueur segment 1` (`KismetMathLibrary.VSize` (- (`SceneComponent.K2_GetComponentLocation` (`self.Ry_1`)) _returnvalue)))
  (set `self.Longueur segment 2` (`KismetMathLibrary.VSize` (- _returnvalue (`SceneComponent.K2_GetComponentLocation` (`self.Ry_3`)))))
  (set `self.Atteinte min robot` (* 7.0 _returnvalue_x))
  (set `self.Atteinte max robot` (* 22.5 _returnvalue_x))
  (set `self.Offset handle scaled` (* (`self.Offset handle`) (`KismetMathLibrary.MakeVector` _returnvalue_x _returnvalue_x _returnvalue_x))))