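; BP_Robot is a three-axis robot arm actor that mirrors and commands a physical robot from a spawned, attached handle.
; CalculerPosition derives base rotation and two joint angles from the handle position by trigonometric inverse kinematics, clamped to reach and angle limits.
; Sendinfo POSTs those angles as VaRest JSON over HTTP and queues the move.
; A looping timer plays queued moves with synchronized joint speeds, driving MSRobot sound parameters.
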(event `self.ReceiveBeginPlay`
  (bind (_offset_handle_scaled_x _offset_handle_scaled_y _offset_handle_scaled_z) (`KismetMathLibrary.BreakVector` (`self.Offset handle scaled`)))
  (bind (_returnvalue_x _returnvalue_y) (`KismetMathLibrary.BreakVector` (`SceneComponent.GetForwardVector` (`self.DefaultSceneRoot`))))
  (bind _output_get (set `self.Position handle` (+ (`SceneComponent.K2_GetComponentLocation` (`self.Ry_3`)) (`KismetMathLibrary.MakeVector` (* _offset_handle_scaled_x _returnvalue_x) (* _offset_handle_scaled_x _returnvalue_y) _offset_handle_scaled_z))))
  (bind _returnvalue (`|SpawnActorFromClass` "/Game/Briques_projets/Grab/Handle_v2/BP_handle_v2.BP_handle_v2_C" (`KismetMathLibrary.MakeTransform` _output_get) "AlwaysSpawn" "OverrideRootScale" self null))
  (`self.K2_AttachToComponent` _returnvalue (`self.Bati`) "None" "KeepWorld" "KeepWorld" "KeepWorld" true)
  (`/Game/Briques_projets/Grab/Handle_v2/BP_handle_v2.Initialisation` _returnvalue null null (`KismetMathLibrary.MakeTransform` (0.0 0.0 0.0) (struct) (0.015 0.015 0.015)) self)
  (bind (_rz _ry1 _ry2) (`self.Calculer Position`))
  (bind _output_get_2 (set `self.Current Rz` _rz))
  (bind _output_get_3 (set `self.Current Ry_1` _ry1))
  (bind _output_get_4 (set `self.Current Ry_2` _ry2))
  (`self.Move robot` _output_get_2 _output_get_3 _output_get_4))

(event `/Game/Briques_projets_rg2/Joueur/BPI_Interractions_VR.TriggerPressed`
  (`self.Send info`))

(event `/Game/Briques_projets_rg2/Joueur/BPI_Interractions_VR.TriggerReleased`)

(event `Send info`
  (bind _returnvalue (subsystem `VaRestSubsystem`))
  (bind _returnvalue_2 (`AudioComponent.GetParameterInterface` (`self.MS_Robot`)))
  (bind (_output_x _output_y _output_z) (`KismetMathLibrary.BreakVector` (`|GetArrayItem` (`self.WaitListMoves`))))
  (bind (_parameters_kinect_lmin _parameters_kinect_lmax _parameters_kinect_hmin _parameters_kinect_hmax _parameters_kinect_dmin _parameters_kinect_dmax _parameters_kinect_nbvalmoy _parameters_kinect_simplification _parameters_kinect_ip) (break `/Game/Briques_projets_rg2/Kinect_webserver/STR_Param_kinect` (`/Game/Briques_projets_rg2/Kinect_webserver/BP_serveur_kinect.Parameters kinect` (`self.Server kinect`))))
  (bind _returnvalue_3 (- _output_x (`self.Current Rz`)))
  (bind _returnvalue_4 (- _output_y (`self.Current Ry_1`)))
  (bind _returnvalue_5 (- _output_z (`self.Current Ry_2`)))
  (bind _returnvalue_6 (/ (`KismetMathLibrary.FMax` (`KismetMathLibrary.Abs` _returnvalue_3) (`KismetMathLibrary.Abs` _returnvalue_4) (`KismetMathLibrary.Abs` _returnvalue_5)) (`self.Max speed robot`)))
  (bind _returnvalue_7 (`KismetMathLibrary.SelectFloat` _returnvalue_6 1000000000.0 (!= _returnvalue_6 0.0)))
  (bind _returnvalue_8 (/ _returnvalue_5 _returnvalue_7))
  (bind _returnvalue_9 (/ _returnvalue_3 _returnvalue_7))
  (bind _returnvalue_10 (/ _returnvalue_4 _returnvalue_7))
  (bind (_rz _ry1 _ry2) (`self.Calculer Position`))
  (set `self.Goal Rz` _rz)
  (set `self.Goal Ry_1` _ry1)
  (set `self.Goal Ry_2` _ry2)
  ;[1 1 1] making JSON and sending it to the robot
  (`|ExecutionSequence`
    (:`then_0`
      (bind _returnvalue_11 (`VaRestSubsystem.ConstructVaRestJsonObject` _returnvalue))
      (bind _output_get (set `self.Json_Position` _returnvalue_11))
      (`VaRestJsonObject.SetIntegerField` _output_get "Rz" (`KismetMathLibrary.FFloor` (* (`self.Goal Rz`) 10.0)))
      (`VaRestJsonObject.SetIntegerField` _output_get "Ry1" (`KismetMathLibrary.FFloor` (* (`self.Goal Ry_1`) 10.0)))
      (`VaRestJsonObject.SetIntegerField` _output_get "Ry2" (`KismetMathLibrary.FFloor` (* (`self.Goal Ry_2`) 10.0))))
    (:`then_1`
      (bind _returnvalue_12 (`VaRestSubsystem.ConstructVaRestJsonObject` _returnvalue))
      (bind _output_get_2 (set `self.Json_var` _returnvalue_12))
      (`VaRestJsonObject.SetObjectField` _output_get_2 "Position" (`self.Json_Position`))
      (`VaRestJsonObject.SetIntegerField` _output_get_2 "SpeedMax" 4000))
    (:`then_2`
      (`VaRestSubsystem.CallURL` _returnvalue (`KismetStringLibrary.Concat_StrStr` "http://" _parameters_kinect_ip ":2021/robot") "POST" "json" (`self.Json_var`) (delegate `ReceptionJson`))
      (`KismetArrayLibrary.Array_Add` (`self.WaitListMoves`) (`KismetMathLibrary.MakeVector` (`self.Goal Rz`) (`self.Goal Ry_1`) (`self.Goal Ry_2`)))
      (if (not (`self.Robot moving`))
        (set `self.Robot moving` true)
        (set `self.V Rz` _returnvalue_9 :!label _label)
        (set `self.V RY_1` _returnvalue_10)
        (set `self.V Ry_2` _returnvalue_8)
        (set `self.temps init` (`GameplayStatics.GetTimeSeconds`))
        (set `self.duree deplacement` _returnvalue_7)
        (`AudioParameterInterface.SetFloatArray` _returnvalue_2 "Frequence" (`|MakeArray` (* (`KismetMathLibrary.Abs` _returnvalue_9) 7.0) (* (`KismetMathLibrary.Abs` _returnvalue_10) 7.0) (* (`KismetMathLibrary.Abs` _returnvalue_8) 7.0)))
        (`AudioParameterInterface.Trigger` _returnvalue_2 "Setup")
        (bind _returnvalue_13 (`KismetSystemLibrary.K2_SetTimerDelegate` (delegate `Robot_move`) 0.013 true))))))

(event `/Game/Briques_projets_rg2/Joueur/BPI_Interractions_VR.APressed`
  (params (`Handle used` :type "Actor Object Reference"))
  (`KismetSystemLibrary.PrintString` "ROBOT : Reception de la pression sur le bouton A"))

(event `ReceptionJson`
  (params (Request :type "VaRestRequestJSON Object Reference"))
  ;[1 1 1] making JSON and sending it to the robot
  (switch `EVaRestRequestStatus` (`VaRestRequestJSON.GetStatus` Request)
    (:`Failed`
      _)
    (:`Failed_ConnectionError`
      _))
  (`KismetSystemLibrary.PrintString` "erreur de connexion"))

(event `/Game/Briques_projets_rg2/Joueur/BPI_Interractions_VR.BPressed`
  (params (`Handle used` :type "Actor Object Reference"))
  (`KismetSystemLibrary.PrintString` "ROBOT : Reception de la pression sur le bouton B"))

(event `Robot_move`
  (bind _returnvalue (- (`GameplayStatics.GetTimeSeconds`) (`self.temps init`)))
  (bind _returnvalue_2 (+ (`self.Current Ry_2`) (* (`self.V Ry_2`) _returnvalue)))
  (bind _returnvalue_3 (+ (`self.Current Rz`) (* (`self.V Rz`) _returnvalue)))
  (bind _returnvalue_4 (+ (`self.Current Ry_1`) (* (`self.V RY_1`) _returnvalue)))
  (`self.Move robot` _returnvalue_3 _returnvalue_4 _returnvalue_2)
  (if (>= (`GameplayStatics.GetTimeSeconds`) (+ (`self.temps init`) (`self.duree deplacement`)))
    (`|ExecutionSequence`
      (:`then_0`
        (`AudioParameterInterface.Trigger` (`AudioComponent.GetParameterInterface` (`self.MS_Robot`)) "Stop"))
      (:`then_1`
        (`KismetSystemLibrary.K2_ClearAndInvalidateTimerHandle` (stale `Send info` _returnvalue_13)))
      (:`then_2`
        (set `self.Current Rz` _returnvalue_3)
        (set `self.Current Ry_1` _returnvalue_4)
        (set `self.Current Ry_2` _returnvalue_2))
      (:`then_3`
        (`KismetArrayLibrary.Array_Remove` (`self.WaitListMoves`)))
      (:`then_4`
        (if (> (`KismetArrayLibrary.Array_Length` (`self.WaitListMoves`)) 0)
          (goto _label)
          (else
            (set `self.Robot moving` false)))))))

(fn `Calculer Position`
  (returns (Rz :type "Float (double-precision)") (Ry1 :type "Float (double-precision)") (Ry2 :type "Float (double-precision)"))
  (bind (_offset_handle_scaled_x _offset_handle_scaled_y _offset_handle_scaled_z) (`KismetMathLibrary.BreakVector` (`self.Offset handle scaled`)))
  (bind _bati (`self.Bati`))
  (bind _longueur_segment_2 (`self.Longueur segment 2`))
  (bind _longueur_segment_1 (`self.Longueur segment 1`))
  (bind _longueur_segment_1_2 (`self.Longueur segment 1`))
  (bind _returnvalue (`KismetMathLibrary.ProjectVectorOnToPlane` (- (`self.Position handle`) (`SceneComponent.K2_GetComponentLocation` (`self.Bati`))) (`SceneComponent.GetUpVector` (`self.Bati`))))
  (bind (_returnvalue_x _returnvalue_y) (`KismetMathLibrary.BreakVector` (`KismetMathLibrary.Normal` (`KismetMathLibrary.ProjectVectorOnToPlane` (- (`self.Position handle`) (`SceneComponent.K2_GetComponentLocation` (`self.Bati`))) (`KismetMathLibrary.GetUpVector` (`SceneComponent.K2_GetComponentRotation` (`self.Bati`)))) 0.001)))
  (bind _returnvalue_2 (- (- (`self.Position handle`) (`SceneComponent.K2_GetComponentLocation` (`self.Ry_1`))) (`KismetMathLibrary.MakeVector` (* _offset_handle_scaled_x _returnvalue_x) (* _offset_handle_scaled_x _returnvalue_y) _offset_handle_scaled_z)))
  (bind _returnvalue_3 (`KismetMathLibrary.VSize` _returnvalue_2))
  (bind _returnvalue_4 (/ (`self.Atteinte min robot`) _returnvalue_3))
  (bind _returnvalue_5 (/ (`self.Atteinte max robot`) _returnvalue_3))
  (bind _returnvalue_6 (`KismetMathLibrary.SelectVector` (* _returnvalue_2 (`KismetMathLibrary.MakeVector` _returnvalue_4 _returnvalue_4 _returnvalue_4)) (`KismetMathLibrary.SelectVector` (* _returnvalue_2 (`KismetMathLibrary.MakeVector` _returnvalue_5 _returnvalue_5 _returnvalue_5)) _returnvalue_2 (> _returnvalue_3 (`self.Atteinte max robot`))) (< _returnvalue_3 (`self.Atteinte min robot`))))
  (bind _returnvalue_7 (`KismetMathLibrary.VSize` _returnvalue_6))
  (bind _returnvalue_8 (`KismetMathLibrary.ClampAngle` (- 0.0 (`KismetMathLibrary.DegAsin` (/ (`KismetMathLibrary.Dot_VectorVector` _returnvalue_6 (`SceneComponent.GetUpVector` (`self.Bati`))) (`KismetMathLibrary.VSize` _returnvalue_6))) (`KismetMathLibrary.DegAcos` (/ (- (`KismetMathLibrary.Square` (`self.Longueur segment 2`)) (`KismetMathLibrary.Square` _returnvalue_7) (`KismetMathLibrary.Square` _longueur_segment_1_2)) (* _returnvalue_7 _longueur_segment_1_2 -2.0)))) 223.0 345.0))
  (return (`KismetMathLibrary.FClamp` (* (`KismetMathLibrary.DegAcos` (/ (`KismetMathLibrary.Dot_VectorVector` _returnvalue (`SceneComponent.GetForwardVector` _bati)) (`KismetMathLibrary.VSize` _returnvalue))) (`KismetMathLibrary.SelectFloat` 1.0 -1.0 (> (`KismetMathLibrary.Dot_VectorVector` _returnvalue (`SceneComponent.GetRightVector` _bati)) 0.0))) -90.0 90.0) (+ _returnvalue_8 180.0) (+ _returnvalue_8 (`KismetMathLibrary.FClamp` (`KismetMathLibrary.DegAcos` (/ (- (`KismetMathLibrary.Square` (`KismetMathLibrary.VSize` _returnvalue_6)) (`KismetMathLibrary.Square` _longueur_segment_1) (`KismetMathLibrary.Square` _longueur_segment_2)) (* _longueur_segment_1 _longueur_segment_2 2.0))) (`KismetMathLibrary.FMax` (- 0.0 _returnvalue_8 23.0) 40.0) (`KismetMathLibrary.FMin` (- 0.0 _returnvalue_8 -90.0) 140.0)))))

(fn `Communicate_data_handle`
  (params (Position :type "Vector Structure") (Rotation :type "Rotator Structure") (`Ref handle` :type "/Game/Briques_projets/Grab/Handle_v2/BP_handle_v2 Object Reference") (`Object to move` :type "Actor Object Reference"))
  (returns (`Controlled by target` :type Boolean))
  (locals (X :type "Float (double-precision)" :default 0.0))
  (bind _robot_ghost (`self.Robot ghost`))
  (`/Engine/EditorBlueprintResources/StandardMacros.IsValid` _robot_ghost
    (:`Is Valid`
      (message `/Game/Briques_projets/Grab/Handle_v2/BPi_Grab.Communicate_data_handle` _robot_ghost Position (struct) null null))
    (:`Is Not Valid`
      _))
  (set `self.Position handle` Position)
  (return false))

(fn `Define_focus`
  (params (Focus :type Boolean))
  (returns (Ok :type Boolean))
  (if Focus
    (`/Engine/EditorBlueprintResources/StandardMacros.IsValid` (`self.Robot ghost`)
      (:`Is Valid`
        (`self.K2_DestroyActor` (`self.Robot ghost`)))
      (:`Is Not Valid`
        _))
    (bind _returnvalue (`|SpawnActorFromClass` "/Game/Briques_projets_rg2/Robot/BP_Robot_ghost.BP_Robot_ghost_C" (`KismetMathLibrary.MakeTransform` (0.0 0.0 0.0)) "Undefined" "OverrideRootScale" null null))
    (bind _output_get (set `self.Robot ghost` _returnvalue))
    (`self.K2_AttachToComponent` _output_get (`self.DefaultSceneRoot`) "None" "KeepRelative" "KeepRelative" "KeepRelative" true)
    (else
      (`self.K2_DestroyActor` (`self.Robot ghost`))
      (`self.Send info`)))
  (return true))

(fn `Get_handle_details`
  (returns (`Is grabbable` :type Boolean) (`Is Grabbed` :type Boolean))
  (return false false))

(fn `IsHeld`
  (returns (bHeld :type Boolean) (AttachedToParent :type "SceneComponent Object Reference"))
  (return false null))

(fn `Move robot`
  (params (Rz :type "Float (double-precision)") (Ry_1 :type "Float (double-precision)") (Ry_2 :type "Float (double-precision)"))
  (bind _returnvalue (- Ry_1 180.0))
  (bind _returnvalue_2 (- Ry_2 _returnvalue))
  (`SceneComponent.K2_SetRelativeRotation` (`self.Rz`) (`KismetMathLibrary.MakeRotator` 0.0 0.0 Rz) false false)
  (`SceneComponent.K2_SetRelativeRotation` (`self.Rz_pignon`) (`KismetMathLibrary.MakeRotator` 0.0 0.0 (* Rz -3.5555)) false false)
  (`SceneComponent.K2_SetRelativeRotation` (`self.Ry_1`) (`KismetMathLibrary.MakeRotator` 0.0 0.0 _returnvalue) false false)
  (`SceneComponent.K2_SetRelativeRotation` (`self.Ry_1-2`) (`KismetMathLibrary.MakeRotator` 0.0 0.0 _returnvalue) false false)
  (`SceneComponent.K2_SetRelativeRotation` (`self.Ry_2-2`) (`KismetMathLibrary.MakeRotator` 0.0 0.0 (- 0.0 _returnvalue)) false false)
  (`SceneComponent.K2_SetRelativeRotation` (`self.Ry_2`) (`KismetMathLibrary.MakeRotator` 0.0 0.0 _returnvalue_2) false false)
  (`SceneComponent.K2_SetRelativeRotation` (`self.Ry_1-3`) (`KismetMathLibrary.MakeRotator` 0.0 0.0 (+ _returnvalue _returnvalue_2)) false false)
  (`SceneComponent.K2_SetRelativeRotation` (`self.Ry_1-4`) (`KismetMathLibrary.MakeRotator` 0.0 0.0 (- 0.0 _returnvalue_2)) false false)
  (`SceneComponent.K2_SetRelativeRotation` (`self.Ry_2-3`) (`KismetMathLibrary.MakeRotator` 0.0 0.0 (+ _returnvalue _returnvalue_2)) false false)
  (`SceneComponent.K2_SetRelativeRotation` (`self.R_pignon_1`) (`KismetMathLibrary.MakeRotator` 0.0 0.0 (* _returnvalue -3.5555)) false false)
  (`SceneComponent.K2_SetRelativeRotation` (`self.R_pignon_2`) (`KismetMathLibrary.MakeRotator` 0.0 0.0 (* (+ _returnvalue _returnvalue_2) -3.5555)) false false)
  (`SceneComponent.K2_SetRelativeRotation` (`self.Ry_3`) (`KismetMathLibrary.MakeRotator` 0.0 0.0 (- 0.0 _returnvalue _returnvalue_2)) false false))

(fn `Use_handle`
  (params (Grabbed :type Boolean) (`Is selected` :type Boolean) (`Grabed by` :type "StaticMeshComponent Object Reference"))
  (returns (`Object to move` :type "Actor Object Reference") (`Handle's target` :type "Actor Object Reference"))
  (return null null))

(fn `UserConstructionScript`
  (bind _returnvalue_x (`KismetMathLibrary.BreakVector` (`SceneComponent.K2_GetComponentScale` (`self.DefaultSceneRoot`))))
  (bind _returnvalue (`SceneComponent.K2_GetComponentLocation` (`self.Ry_2`)))
  (set `self.Longueur segment 1` (`KismetMathLibrary.VSize` (- (`SceneComponent.K2_GetComponentLocation` (`self.Ry_1`)) _returnvalue)))
  (set `self.Longueur segment 2` (`KismetMathLibrary.VSize` (- _returnvalue (`SceneComponent.K2_GetComponentLocation` (`self.Ry_3`)))))
  (set `self.Atteinte min robot` (* 7.0 _returnvalue_x))
  (set `self.Atteinte max robot` (* 22.5 _returnvalue_x))
  (set `self.Offset handle scaled` (* (`self.Offset handle`) (`KismetMathLibrary.MakeVector` _returnvalue_x _returnvalue_x _returnvalue_x)))
  (set `self.hauteur min` (* -5.0 _returnvalue_x)))